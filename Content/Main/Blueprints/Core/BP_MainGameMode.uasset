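; Main game mode that sets up per-map enemies and hazards, pauses on game finish and restarts levels.
; BeginPlay spawns ball enemies by map name, and GetEnemySpawnLocations exposes each map's grid bounds.
; Looping timers activate random inactive spikes on Map 0 and, on Maps 0 and 1, spawn spike balls, replacing tagged bouncing balls in place while any remain.
; It also saves and loads registered names through BP_Saver.
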(event `self.ReceiveBeginPlay`
  (bind _returnvalue (`GameplayStatics.GetPlayerController` 0))
  (bind _returnvalue_2 (`GameplayStatics.CreateSaveGameObject` "/Game/Main/Blueprints/Core/BP_Saver.BP_Saver_C"))
  (set `self.SaveRef` _returnvalue_2)
  (set `PlayerController.bShowMouseCursor` false _returnvalue)
  (`WidgetBlueprintLibrary.SetInputMode_GameOnly` _returnvalue)
  (`self.SetUpVariables`)
  (`self.SpawnEnemies`)
  (bind _outactors (`GameplayStatics.GetAllActorsOfClassWithTag` "/Game/Main/Blueprints/Enemies/BP_BouncingBaseBallEnemy.BP_BouncingBaseBallEnemy_C" "Parent"))
  (set `self.BouncingBalls` _outactors)
  (`self.StartSpikesSpawn`)
  (`self.StartSpikeBallSpawn`))

(event `StartSpikesSpawn`
  (bind _returnvalue (`GameplayStatics.GetCurrentLevelName` true))
  (switch `string` _returnvalue
    (:`Map0`
      (set `self.MaxSpikesCount` (`KismetMathLibrary.Round` (* (`self.MaxSpikesPercent`) (`self.MaxSpikesCount`))))
      (bind _outactors (`GameplayStatics.GetAllActorsOfClass` "/Game/Main/Blueprints/Obstacles/BP_Spikes.BP_Spikes_C"))
      (set `self.Spikes` _outactors)
      (`KismetSystemLibrary.K2_SetTimer` null "AddActiveSpike" (`self.SpawnSpikesTimer`) true))))

(event `SetUpVariables`
  (bind _returnvalue (`GameplayStatics.GetCurrentLevelName` true))
  (switch `string` _returnvalue
    (:`Map1`
      (set `self.SpawnSpikeBallsTime` 5.0))))

(event `StartSpikeBallSpawn`
  (bind _returnvalue (`GameplayStatics.GetCurrentLevelName` true))
  (switch `string` _returnvalue
    (:`Map0`
      _)
    (:`Map1`
      _))
  (`KismetSystemLibrary.K2_SetTimer` null "SpawnSpikeBall" (`self.SpawnSpikeBallsTime`) true))

(event `AddActiveSpike`
  (if (> (`self.MaxSpikesCount`) 0)
    (`/Engine/EditorBlueprintResources/StandardMacros.DecrementInt` (`self.MaxSpikesCount`)
      (:`  `
        (`self.SpawnSpike`)))
    (else
      (`KismetSystemLibrary.K2_ClearTimer` null "AddActiveSpike"))))

(event `FinishGame`
  (params (Score :type "Float (double-precision)"))
  (set `self.IsGameFinished` true)
  (`GameplayStatics.SetGamePaused` true)
  (`self.SetFinalScore` Score))

(event `RestartGame`
  (bind _returnvalue (`GameplayStatics.GetCurrentLevelName` true))
  (`GameplayStatics.OpenLevel` (`KismetStringLibrary.Conv_StringToName` _returnvalue)))

(fn `GetEnemySpawnLocations`
  (returns (CellCount :type Integer) (MinCoords :type "Vector Structure"))
  (bind _returnvalue (`GameplayStatics.GetCurrentLevelName` true))
  (switch `string` _returnvalue
    (:`Map0`
      (return (`self.Map0_CellCount`) (`self.Map0_MinCoords`)))
    (:`Map1`
      (return (`self.Map1_CellCount`) (`self.Map1_MinCoords`)))
    (:`Map69`
      (return (`self.Map69_CellCount`) (`self.Map69_MinCoords`)))))

(fn `LoadGame`
  (bind _returnvalue (`GameplayStatics.DoesSaveGameExist` (`self.SlotSave`)))
  (if _returnvalue
    (bind _returnvalue_2 (`GameplayStatics.LoadGameFromSlot` (`self.SlotSave`)))
    (set `self.SaveRef` _returnvalue_2)
    (else
      (bind _returnvalue_3 (`GameplayStatics.CreateSaveGameObject` "/Game/Main/Blueprints/Core/BP_Saver.BP_Saver_C"))
      (set `self.SaveRef` _returnvalue_3)))
  (bind _asbp_saver (cast `/Game/Main/Blueprints/Core/BP_Saver` (`self.SaveRef`)))
  (set `self.RRegisteredNames` (`/Game/Main/Blueprints/Core/BP_Saver.RegisteredNames` _asbp_saver)))

(fn `Save Game`
  (params (WRegisteredNames :type "Array of String"))
  (bind _returnvalue (`GameplayStatics.DoesSaveGameExist` (`self.SlotSave`)))
  (if _returnvalue
    (bind _returnvalue_2 (`GameplayStatics.LoadGameFromSlot` (`self.SlotSave`)))
    (set `self.SaveRef` _returnvalue_2)
    (else
      (bind _returnvalue_3 (`GameplayStatics.CreateSaveGameObject` "/Game/Main/Blueprints/Core/BP_Saver.BP_Saver_C"))
      (set `self.SaveRef` _returnvalue_3)))
  (bind _asbp_saver (cast `/Game/Main/Blueprints/Core/BP_Saver` (`self.SaveRef`)))
  (set `/Game/Main/Blueprints/Core/BP_Saver.RegisteredNames` (`local.WRegisteredNames`) _asbp_saver)
  (`GameplayStatics.SaveGameToSlot` (`self.SaveRef`) (`self.SlotSave`)))

(fn `SpawnEnemies`
  (locals (BlueBallCount :type Integer) (PinkBallCount :type Integer))
  (bind _returnvalue (`GameplayStatics.GetCurrentLevelName` true))
  (switch `string` _returnvalue
    (:`Map0`
      (set `local.BlueBallCount` (`self.Map0_BlueBallCount`))
      (set `local.PinkBallCount` (`self.Map0_PinkBallCount`)))
    (:`Map1`
      (set `local.BlueBallCount` (`self.Map1_BlueBallCount`))
      (set `local.PinkBallCount` (`self.Map1_PinkBallCount`)))
    (:`Map69`
      (set `local.BlueBallCount` (`self.Map69_BlueBallCount`))
      (set `local.PinkBallCount` (`self.Map69_PinkBallCount`))))
  (for _ (range 1 (+ (`local.BlueBallCount`) 1))
    (`|SpawnActorFromClass` "/Game/Main/Blueprints/Enemies/BP_BaseBallEnemy.BP_BaseBallEnemy_C" (`KismetMathLibrary.MakeTransform` (0.0 0.0 0.0)) "AlwaysSpawn" "MultiplyWithRoot" null null))
  (for _ (range 1 (+ (`local.PinkBallCount`) 1))
    (bind _returnvalue_2 (`GameplayStatics.GetCurrentLevelName` true))
    (switch `string` _returnvalue_2
      (:`Map0`
        (`|SpawnActorFromClass` "/Game/Main/Blueprints/Enemies/BP_BouncingBaseBallEnemy.BP_BouncingBaseBallEnemy_C" (`KismetMathLibrary.MakeTransform` (0.0 0.0 0.0)) "AlwaysSpawn" "MultiplyWithRoot" null null :!label _label))
      (:`Map1`
        (`|SpawnActorFromClass` "/Game/Main/Blueprints/Enemies/BP_SpikeBallEnemy.BP_SpikeBallEnemy_C" (`KismetMathLibrary.MakeTransform` (0.0 0.0 0.0)) "AlwaysSpawn" "MultiplyWithRoot" null null))
      (:`Map69`
        (goto _label)))))

(fn `SpawnSpike`
  (locals (RandomSpikeInd :type Integer) (RandomSpike :type "/Game/Main/Blueprints/Obstacles/BP_Spikes Object Reference"))
  (bind _spikes (`self.Spikes`))
  (`KismetArrayLibrary.Array_Shuffle` _spikes)
  (for _array_element _spikes
    (if (not (`/Game/Main/Blueprints/Obstacles/BP_Spikes.IsSpikeActive` _array_element))
      (`/Game/Main/Blueprints/Obstacles/BP_Spikes.AutoActivateSpike` _array_element)
      (break))))

(fn `SpawnSpikeBall`
  (locals (PrevLocation :type "Vector Structure"))
  (bind _output (`|GetArrayItem` (`self.BouncingBalls`) (`self.BounceBallind`)))
  (if (>= (`self.BounceBallind`) (`KismetArrayLibrary.Array_Length` (`self.BouncingBalls`)))
    (`|SpawnActorFromClass` "/Game/Main/Blueprints/Enemies/BP_SpikeBallEnemy.BP_SpikeBallEnemy_C" (`KismetMathLibrary.MakeTransform` (0.0 0.0 0.0)) "AlwaysSpawn" "MultiplyWithRoot" null null)
    (else
      (set `local.PrevLocation` (`self.K2_GetActorLocation` _output))
      (`self.K2_DestroyActor` _output)
      (`/Engine/EditorBlueprintResources/StandardMacros.IncrementInt` (`self.BounceBallind`)
        (:`  `
          (bind _returnvalue (`|SpawnActorFromClass` "/Game/Main/Blueprints/Enemies/BP_SpikeBallEnemy.BP_SpikeBallEnemy_C" (`KismetMathLibrary.MakeTransform` (0.0 0.0 0.0)) "AlwaysSpawn" "MultiplyWithRoot" null null))
          (`self.K2_SetActorLocation` _returnvalue (`local.PrevLocation`) false true))))))

(fn `UserConstructionScript`)