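; BP_SetUpMainGameMod is a configuration Blueprint that hands its own match settings to BP_MainGameMode.
; Its SetUpVariables function casts the current game mode, stops if that fails, and copies each value across.
; The settings cover ball counts, map layout, purple ball and spike spawning, controls appearance timing and a mobile arena flag.
; The construction script is empty, and nothing within the file calls the function.
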(fn `SetUpVariables`
  (bind _asbp_main_game_mode (cast `/Game/Main/Blueprints/Core/BP_MainGameMode` (`GameplayStatics.GetGameMode`)))
  (set `/Game/Main/Blueprints/Core/BP_MainGameMode.BlueBallCount` (`self.BlueBallCount`) _asbp_main_game_mode)
  (set `/Game/Main/Blueprints/Core/BP_MainGameMode.PinkBallCount` (`self.PinkBallCount`) _asbp_main_game_mode)
  (set `/Game/Main/Blueprints/Core/BP_MainGameMode.PurpleBallCount` (`self.PurpleBallCount`) _asbp_main_game_mode)
  (set `/Game/Main/Blueprints/Core/BP_MainGameMode.MapCellCount` (`self.MapCellCount`) _asbp_main_game_mode)
  (set `/Game/Main/Blueprints/Core/BP_MainGameMode.MapMinCoords` (`self.MapMinCoords`) _asbp_main_game_mode)
  (set `/Game/Main/Blueprints/Core/BP_MainGameMode.DoesSpawnPurpleBalls` (`self.DoesSpawnPurpleBalls`) _asbp_main_game_mode)
  (set `/Game/Main/Blueprints/Core/BP_MainGameMode.DoesSpawnSpikes` (`self.DoesSpawnSpikes`) _asbp_main_game_mode)
  (set `/Game/Main/Blueprints/Core/BP_MainGameMode.SpawnPurpleBallsTime` (`self.SpawnPurpleBallsTime`) _asbp_main_game_mode)
  (set `/Game/Main/Blueprints/Core/BP_MainGameMode.ControlsAppearanceTime` (`self.ContolsAppearanceTime`) _asbp_main_game_mode)
  (set `/Game/Main/Blueprints/Core/BP_MainGameMode.SpawnSpikesTime` (`self.SpawnSpikesTime`) _asbp_main_game_mode)
  (set `/Game/Main/Blueprints/Core/BP_MainGameMode.IsArenaMobile` (`self.IsArenaMobile`) _asbp_main_game_mode))

(fn `UserConstructionScript`)