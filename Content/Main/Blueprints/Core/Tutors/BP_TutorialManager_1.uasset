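; Tutorial manager for the first tutorial map, stepping the player through a sequence of missions that ends by opening MapTutor2.
; It binds to the player's kill, energy, descent and score events, using trigger flags and goal counters to advance from first kill through energy, mid-flight kills, shotgun kills and score.
; Each mission swaps the tutorial card widget, spawns or destroys ball enemies, and gradually unlocks shotgun and score display.
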(event `self.ReceiveBeginPlay`
  (`self.SetUpWidgets`)
  (bind _asbp_main_character (cast `/Game/Main/Blueprints/Player/BP_MainCharacter` (`GameplayStatics.GetPlayerCharacter` 0)))
  (bind _output_get (set `self.PlayerRef` _asbp_main_character))
  (set `/Game/Main/Blueprints/Player/BP_MainCharacter.IsShotgunAvailable` false _output_get)
  (bind _asbp_main_player_controller (cast `/Game/Main/Blueprints/Player/BP_MainPlayerController` (`GameplayStatics.GetPlayerController` 0)))
  (set `/Game/Main/Blueprints/Player/BP_MainPlayerController.CanRestart` false _asbp_main_player_controller)
  (set `/Game/Main/Blueprints/Player/BP_MainPlayerController.CanSuicide` false _asbp_main_player_controller)
  (add `/Game/Main/Blueprints/Player/BP_MainCharacter.KilledEnemy` _output_get (delegate `OnKilledEnemy`))
  (add `/Game/Main/Blueprints/Player/BP_MainCharacter.ChangedEnergy` (`self.PlayerRef`) (delegate `OnChangedEnergy`))
  (add `/Game/Main/Blueprints/Player/BP_MainCharacter.OnDescent` (`self.PlayerRef`) (delegate `OnDescent`))
  (add `/Game/Main/Blueprints/Player/BP_MainCharacter.ChangedScore` (`self.PlayerRef`) (delegate `OnChangedScore`)))

(event `OnKilledEnemy`
  (params (IsShot :type Boolean))
  (if (`self.0msTrigger`)
    (set `self.0msTrigger` false)
    (`self.1stMission`)
    (elif (`self.2MsTrigger`)
      (`/Engine/EditorBlueprintResources/StandardMacros.IncrementInt` (`self.2MsMidFlightKill`)
        (:`  `
          (if (== (`self.2MsMidFlightKill`) 2)
            (bind _result (`/Engine/EditorBlueprintResources/StandardMacros.DecrementInt` (`self.2MsGoal`))
              (:`  `
                (bind _aswb_tutor_card_2 (cast `/Game/Main/Blueprints/UI/TutorialCards/WB_TutorCard_2` (`self.TutorCard`)))
                (`/Game/Main/Blueprints/UI/TutorialCards/WB_TutorCard_2.SetGoal` _aswb_tutor_card_2 _result)
                (if (<= (`self.2MsGoal`) 0)
                  (set `self.2MsTrigger` false)
                  (`self.3rdMission`)))))))
      (elif (`self.3MsTrigger`)
        (if IsShot
          (bind _result_2 (`/Engine/EditorBlueprintResources/StandardMacros.DecrementInt` (`self.3MsGoal`))
            (:`  `
              (bind _aswb_tutor_card_3 (cast `/Game/Main/Blueprints/UI/TutorialCards/WB_TutorCard_3` (`self.TutorCard`)))
              (`/Game/Main/Blueprints/UI/TutorialCards/WB_TutorCard_3.SetGoal` _aswb_tutor_card_3 _result_2)
              (if (<= (`self.3MsGoal`) 0)
                (set `self.3MsTrigger` false)
                (`self.4thMission`)))))))))

(event `OnChangedEnergy`
  (params (EnergyVal :type "Float (double-precision)"))
  (if (>= EnergyVal (`self.1MsGoal`))
    (remove `/Game/Main/Blueprints/Player/BP_MainCharacter.ChangedEnergy` (`self.PlayerRef`) (delegate `OnChangedEnergy`))
    (`self.2ndMission`)))

(event `OnDescent`
  (set `self.2MsMidFlightKill` 0))

(event `OnChangedScore`
  (params (Score :type "Float (double-precision)"))
  (if (>= Score (`self.4MsGoal`))
    (`self.5thMission`)))

(event `SetUpWidgets`
  (`KismetSystemLibrary.DelayUntilNextTick`)
  (bind _returnvalue (`|CreateWidget` "/Game/Main/Blueprints/UI/TutorialCards/WB_TutorCard_0.WB_TutorCard_0_C" (`GameplayStatics.GetPlayerController` 0)))
  (bind _output_get (set `self.TutorCard` _returnvalue))
  (`UserWidget.AddToViewport` _output_get 0)
  (bind _asbp_player_hud (cast `/Game/Main/Blueprints/UI/BP_PlayerHUD` (`PlayerController.GetHUD` (`GameplayStatics.GetPlayerController` 0))))
  (bind _output_get_2 (set `self.PlayerHUDRef` _asbp_player_hud))
  (bind _playerui (`/Game/Main/Blueprints/UI/BP_PlayerHUD.PlayerUI` _output_get_2))
  (`/Game/Main/Blueprints/UI/WB_Score.HideScore` (`/Game/Main/Blueprints/UI/WB_PlayerUI.WB_Score` _playerui))
  (`/Game/Main/Blueprints/UI/WB_Combo.UnbindFromPlayer` (`/Game/Main/Blueprints/UI/WB_PlayerUI.WB_Combo` _playerui)))

(event `1stMission`
  (`Widget.RemoveFromParent` (`self.TutorCard`))
  (bind _returnvalue (`|CreateWidget` "/Game/Main/Blueprints/UI/TutorialCards/WB_TutorCard_1.WB_TutorCard_1_C" (`GameplayStatics.GetPlayerController` 0)))
  (bind _output_get (set `self.TutorCard` _returnvalue))
  (`UserWidget.AddToViewport` _output_get 0)
  (`self.SpawnBalls` (- (`self.1MsBlueBallls`) 1) "/Game/Main/Blueprints/Enemies/BP_BaseBallEnemy.BP_BaseBallEnemy_C"))

(event `2ndMission`
  (`Widget.RemoveFromParent` (`self.TutorCard`))
  (bind _returnvalue (`|CreateWidget` "/Game/Main/Blueprints/UI/TutorialCards/WB_TutorCard_2.WB_TutorCard_2_C" (`GameplayStatics.GetPlayerController` 0)))
  (bind _output_get (set `self.TutorCard` _returnvalue))
  (`UserWidget.AddToViewport` _output_get 0)
  (bind _aswb_tutor_card_2 (cast `/Game/Main/Blueprints/UI/TutorialCards/WB_TutorCard_2` (`self.TutorCard`)))
  (`/Game/Main/Blueprints/UI/TutorialCards/WB_TutorCard_2.SetGoal` _aswb_tutor_card_2 (`self.2MsGoal`))
  (set `self.2MsTrigger` true)
  (`self.DestroyBalls` (- (`self.1MsBlueBallls`) (`self.2MsBlueBallls`)) "/Game/Main/Blueprints/Enemies/BP_BaseBallEnemy.BP_BaseBallEnemy_C")
  (`/Game/Main/Blueprints/Player/BP_MainCharacter.ResetEnergy` (`self.PlayerRef`)))

(event `3rdMission`
  (bind _playerref (`self.PlayerRef`))
  (`Widget.RemoveFromParent` (`self.TutorCard`))
  (bind _returnvalue (`|CreateWidget` "/Game/Main/Blueprints/UI/TutorialCards/WB_TutorCard_3.WB_TutorCard_3_C" (`GameplayStatics.GetPlayerController` 0)))
  (bind _output_get (set `self.TutorCard` _returnvalue))
  (`UserWidget.AddToViewport` _output_get 0)
  (bind _aswb_tutor_card_3 (cast `/Game/Main/Blueprints/UI/TutorialCards/WB_TutorCard_3` (`self.TutorCard`)))
  (`/Game/Main/Blueprints/UI/TutorialCards/WB_TutorCard_3.SetGoal` _aswb_tutor_card_3 (`self.3MsGoal`))
  (set `/Game/Main/Blueprints/Player/BP_MainCharacter.IsShotgunAvailable` true _playerref)
  (set `/Game/Main/Blueprints/Player/BP_MainCharacter.HasNotShot` false _playerref)
  (set `self.3MsTrigger` true)
  (`self.SpawnBalls` (- (`self.3MsBlueBallls`) (`self.2MsBlueBallls`)) "/Game/Main/Blueprints/Enemies/BP_BaseBallEnemy.BP_BaseBallEnemy_C"))

(event `4thMission`
  (`Widget.RemoveFromParent` (`self.TutorCard`))
  (bind _returnvalue (`|CreateWidget` "/Game/Main/Blueprints/UI/TutorialCards/WB_TutorCard_4.WB_TutorCard_4_C" (`GameplayStatics.GetPlayerController` 0)))
  (bind _output_get (set `self.TutorCard` _returnvalue))
  (`UserWidget.AddToViewport` _output_get 0)
  (`/Game/Main/Blueprints/UI/WB_Score.ShowScore` (`/Game/Main/Blueprints/UI/WB_PlayerUI.WB_Score` (`/Game/Main/Blueprints/UI/BP_PlayerHUD.PlayerUI` (`self.PlayerHUDRef`))))
  (`self.SpawnBalls` (`self.4MsPinkBalls`) "/Game/Main/Blueprints/Enemies/BP_BouncingBaseBallEnemy.BP_BouncingBaseBallEnemy_C"))

(event `5thMission`
  (`GameplayStatics.OpenLevel` "MapTutor2"))

(fn `DestroyBalls`
  (params (BallCount :type Integer) (BallType :type "/Game/Main/Blueprints/Enemies/BP_BaseBallEnemy Class Reference"))
  (locals (BallCount_ :type Integer))
  (bind _output_get (set `local.BallCount_` BallCount))
  (if (> _output_get 0)
    (bind _outactors (`GameplayStatics.GetAllActorsOfClass` BallType))
    (for _array_element _outactors
      (`/Game/Main/Blueprints/Enemies/Interfaces/BPI_Enemy.DelayedDestroy` _array_element)
      (bind _result (`/Engine/EditorBlueprintResources/StandardMacros.DecrementInt` (`local.BallCount_`))
        (:`  `
          (if (== _result 0)
            (break)))))))

(fn `SpawnBalls`
  (params (BallCount :type Integer) (BallType :type "/Game/Main/Blueprints/Enemies/BP_BaseBallEnemy Class Reference"))
  (locals (BallCount_ :type Integer))
  (bind _output_get (set `local.BallCount_` BallCount))
  (if (> _output_get 0)
    (for _ (range 1 (+ BallCount 1))
      (`|SpawnActorFromClass` BallType (`KismetMathLibrary.MakeTransform` (0.0 0.0 0.0)) "AlwaysSpawn" "MultiplyWithRoot" null null))))

(fn `UserConstructionScript`)