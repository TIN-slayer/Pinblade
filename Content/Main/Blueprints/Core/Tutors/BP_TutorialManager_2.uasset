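; Tutorial manager for the second tutorial stage that steps the player through missions 5 to 7, with death disabled and score and combo UI hidden or unbound.
; It shows the first tutorial card on BeginPlay, then advances on the player's hit event according to remaining HP.
; At 2 HP it swaps cards, spawns spike-ball enemies and starts the game mode's spike spawning; at zero HP it loads the next tutorial map.
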(event `self.ReceiveBeginPlay`
  (`self.SetUpWidgets`)
  (bind _asbp_main_character (cast `/Game/Main/Blueprints/Player/BP_MainCharacter` (`GameplayStatics.GetPlayerCharacter` 0)))
  (bind _output_get (set `self.PlayerRef` _asbp_main_character))
  (bind _asbp_main_game_mode (cast `/Game/Main/Blueprints/Core/BP_MainGameMode` (`GameplayStatics.GetGameMode`)))
  (set `self.GameModeRef` _asbp_main_game_mode)
  (`self.5thMission`)
  (set `/Game/Main/Blueprints/Player/BP_MainCharacter.CanDie` false _output_get)
  (add `/Game/Main/Blueprints/Player/BP_MainCharacter.GotHIt` _output_get (delegate `OnGotHit`)))

(event `OnGotHit`
  (params (HP :type Integer))
  (if (== HP 2)
    (`self.6thMission`)
    (elif (<= HP 0)
      (`self.7thMission`))))

(event `SetUpWidgets`
  (`KismetSystemLibrary.DelayUntilNextTick`)
  (bind _asbp_player_hud (cast `/Game/Main/Blueprints/UI/BP_PlayerHUD` (`PlayerController.GetHUD` (`GameplayStatics.GetPlayerController` 0))))
  (bind _output_get (set `self.PlayerHUDRef` _asbp_player_hud))
  (bind _playerui (`/Game/Main/Blueprints/UI/BP_PlayerHUD.PlayerUI` _output_get))
  (`/Game/Main/Blueprints/UI/WB_Score.HideScore` (`/Game/Main/Blueprints/UI/WB_PlayerUI.WB_Score` _playerui))
  (`/Game/Main/Blueprints/UI/WB_Combo.UnbindFromPlayer` (`/Game/Main/Blueprints/UI/WB_PlayerUI.WB_Combo` _playerui)))

(event `5thMission`
  (bind _returnvalue (`|CreateWidget` "/Game/Main/Blueprints/UI/TutorialCards/WB_TutorCard_5.WB_TutorCard_5_C" (`GameplayStatics.GetPlayerController` 0)))
  (bind _output_get (set `self.TutorCard` _returnvalue))
  (`UserWidget.AddToViewport` _output_get 0))

(event `6thMission`
  (bind _gamemoderef (`self.GameModeRef`))
  (`Widget.RemoveFromParent` (`self.TutorCard`))
  (bind _returnvalue (`|CreateWidget` "/Game/Main/Blueprints/UI/TutorialCards/WB_TutorCard_6.WB_TutorCard_6_C" (`GameplayStatics.GetPlayerController` 0)))
  (bind _output_get (set `self.TutorCard` _returnvalue))
  (`UserWidget.AddToViewport` _output_get 0)
  (`self.SpawnBalls` (`self.6MsPurpleBalls`) "/Game/Main/Blueprints/Enemies/BP_SpikeBallEnemy.BP_SpikeBallEnemy_C")
  (set `/Game/Main/Blueprints/Core/BP_MainGameMode.DoesSpawnSpikes` true _gamemoderef)
  (`/Game/Main/Blueprints/Core/BP_MainGameMode.StartSpikesSpawn` _gamemoderef))

(event `7thMission`
  (`GameplayStatics.OpenLevel` "MapTutor3"))

(fn `DestroyBalls`
  (params (BallCount :type Integer) (BallType :type "/Game/Main/Blueprints/Enemies/BP_BaseBallEnemy Class Reference"))
  (locals (BallCount_ :type Integer))
  (bind _output_get (set `local.BallCount_` BallCount))
  (if (> _output_get 0)
    (bind _outactors (`GameplayStatics.GetAllActorsOfClass` BallType))
    (for _array_element _outactors
      (`/Game/Main/Blueprints/Enemies/Interfaces/BPI_Enemy.DelayedDestroy` _array_element)
      (bind _result (`/Engine/EditorBlueprintResources/StandardMacros.DecrementInt` (`local.BallCount_`))
        (:`  `
          (if (== _result 0)
            (break)))))))

(fn `SpawnBalls`
  (params (BallCount :type Integer) (BallType :type "/Game/Main/Blueprints/Enemies/BP_BaseBallEnemy Class Reference"))
  (locals (BallCount_ :type Integer))
  (bind _output_get (set `local.BallCount_` BallCount))
  (if (> _output_get 0)
    (for _ (range 1 (+ BallCount 1))
      (`|SpawnActorFromClass` BallType (`KismetMathLibrary.MakeTransform` (0.0 0.0 0.0)) "AlwaysSpawn" "MultiplyWithRoot" null null))))

(fn `UserConstructionScript`)