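; Tutorial manager that runs the eighth tutorial mission, a combo challenge, with player death, restart and suicide disabled.
; On BeginPlay it shows the mission card and binds to the player's hit and combo events, restarting the game when HP runs out.
; Reaching the goal combo swaps the card for the tutorial endgame screen, hides the HUD and pauses.
; Helper functions spawn and destroy balls but go uncalled here.
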(event `self.ReceiveBeginPlay`
  (bind _asbp_main_character (cast `/Game/Main/Blueprints/Player/BP_MainCharacter` (`GameplayStatics.GetPlayerCharacter` 0)))
  (bind _output_get (set `self.PlayerRef` _asbp_main_character))
  (bind _asbp_main_player_controller (cast `/Game/Main/Blueprints/Player/BP_MainPlayerController` (`GameplayStatics.GetPlayerController` 0)))
  (set `/Game/Main/Blueprints/Player/BP_MainPlayerController.CanRestart` false _asbp_main_player_controller)
  (set `/Game/Main/Blueprints/Player/BP_MainPlayerController.CanSuicide` false _asbp_main_player_controller)
  (bind _asbp_main_game_mode (cast `/Game/Main/Blueprints/Core/BP_MainGameMode` (`GameplayStatics.GetGameMode`)))
  (set `self.GameModeRef` _asbp_main_game_mode)
  (`self.8thMission`)
  (set `/Game/Main/Blueprints/Player/BP_MainCharacter.CanDie` false _output_get)
  (add `/Game/Main/Blueprints/Player/BP_MainCharacter.GotHIt` _output_get (delegate `OnGotHit`))
  (add `/Game/Main/Blueprints/Player/BP_MainCharacter.ChangedCombo` _output_get (delegate `OnChangedCombo`)))

(event `OnGotHit`
  (params (HP :type Integer))
  (if (<= HP 0)
    (`/Game/Main/Blueprints/Core/BP_MainGameMode.RestartGame` (`self.GameModeRef`))))

(event `OnChangedCombo`
  (params (ComboCount :type Integer) (ComboTime :type "Float (double-precision)"))
  (if (`self.8MsTrigger`)
    (if (== ComboCount (`self.8MsGoal`))
      (set `self.8MsTrigger` false)
      (`self.FinishTutotial`))))

(event `8thMission`
  (bind _returnvalue (`|CreateWidget` "/Game/Main/Blueprints/UI/TutorialCards/WB_TutorCard_8.WB_TutorCard_8_C" (`GameplayStatics.GetPlayerController` 0)))
  (bind _output_get (set `self.TutorCard` _returnvalue))
  (`UserWidget.AddToViewport` _output_get 0))

(event `FinishTutotial`
  (`Widget.RemoveFromParent` (`self.TutorCard`))
  (bind _asbp_player_hud (cast `/Game/Main/Blueprints/UI/BP_PlayerHUD` (`PlayerController.GetHUD` (`GameplayStatics.GetPlayerController` 0))))
  (set `Widget.Visibility` "Hidden" (`/Game/Main/Blueprints/UI/BP_PlayerHUD.PlayerUI` _asbp_player_hud))
  (`GameplayStatics.SetGamePaused` true)
  (bind _returnvalue (`|CreateWidget` "/Game/Main/Blueprints/UI/TutorialCards/WB_TutorEndgame.WB_TutorEndgame_C" (`GameplayStatics.GetPlayerController` 0)))
  (`UserWidget.AddToViewport` _returnvalue 0))

(fn `DestroyBalls`
  (params (BallCount :type Integer) (BallType :type "/Game/Main/Blueprints/Enemies/BP_BaseBallEnemy Class Reference"))
  (locals (BallCount_ :type Integer))
  (bind _output_get (set `local.BallCount_` BallCount))
  (if (> _output_get 0)
    (bind _outactors (`GameplayStatics.GetAllActorsOfClass` BallType))
    (for _array_element _outactors
      (`/Game/Main/Blueprints/Enemies/Interfaces/BPI_Enemy.DelayedDestroy` _array_element)
      (bind _result (`/Engine/EditorBlueprintResources/StandardMacros.DecrementInt` (`local.BallCount_`))
        (:`  `
          (if (== _result 0)
            (break)))))))

(fn `SpawnBalls`
  (params (BallCount :type Integer) (BallType :type "/Game/Main/Blueprints/Enemies/BP_BaseBallEnemy Class Reference"))
  (locals (BallCount_ :type Integer))
  (bind _output_get (set `local.BallCount_` BallCount))
  (if (> _output_get 0)
    (for _ (range 1 (+ BallCount 1))
      (`|SpawnActorFromClass` BallType (`KismetMathLibrary.MakeTransform` (0.0 0.0 0.0)) "AlwaysSpawn" "MultiplyWithRoot" null null))))

(fn `UserConstructionScript`)