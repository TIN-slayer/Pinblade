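; Base ball enemy that, when killed, plays explosion sound and sparks, then respawns at a random point instead of being destroyed.
; SetUp reads a 3D spawn grid from BP_MainGameMode, from which respawn picks cells on a 100-unit step.
; Respawn hides and teleports the enemy, then retries on following ticks until sphere overlap checks find a clear spot to reveal it.
; Getters expose enemy identity, energy reward, active and armor states.
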(event `self.ReceiveBeginPlay`
  (`self.SetUp`)
  (if (`self.DoStartRespawn`)
    (`self.RandomRespawn`)))

(event `SetUp`
  (bind _asbp_main_game_mode (cast `/Game/Main/Blueprints/Core/BP_MainGameMode` (`GameplayStatics.GetGameMode`)))
  (bind (_cellcount _mincoords) (`/Game/Main/Blueprints/Core/BP_MainGameMode.GetEnemySpawnLocations` _asbp_main_game_mode))
  (set `self.MaxCell` (- _cellcount (`self.MinCell`)))
  (set `self.StartCoords` _mincoords))

(event `RandomRespawn`
  (`self.Hide`)
  (bind _spawnpos (`self.Get Random Spawn Pos`))
  (`self.K2_TeleportTo` _spawnpos)
  (`KismetSystemLibrary.DelayUntilNextTick`)
  (bind _isspottaken (`self.CheckSpawnSpot`))
  (if _isspottaken
    (`self.RandomRespawn`)
    (else
      (`self.Reveal`))))

(event `/Game/Main/Blueprints/Enemies/BPI_EnemyDeath.GetKilled`
  (`self.SpawnAfterDestroySystems`)
  (`self.RandomRespawn`))

(event `Hide`
  (`PrimitiveComponent.SetCollisionEnabled` (`self.Collider`) "NoCollision")
  (`SceneComponent.SetHiddenInGame` (`self.Sphere`) true false))

(event `SpawnAfterDestroySystems`
  (`GameplayStatics.PlaySoundAtLocation` "/Game/Main/Audio/SFX/EnemyExplosion.EnemyExplosion" (`self.K2_GetActorLocation`) (struct) 1.0 1.0 0.0 null null null null)
  (`NiagaraFunctionLibrary.SpawnSystemAtLocation` (`self.DeathSparks`) (`SceneComponent.K2_GetComponentLocation` (`self.Collider`)) (struct) (1.0 1.0 1.0) false))

(event `Reveal`
  (`PrimitiveComponent.SetCollisionEnabled` (`self.Collider`) "QueryAndPhysics")
  (`SceneComponent.SetHiddenInGame` (`self.Sphere`) false true))

(fn `CheckSpawnSpot`
  (returns (IsSpotTaken :type Boolean))
  (bind (_outactors _returnvalue) (`KismetSystemLibrary.SphereOverlapActors` (`self.K2_GetActorLocation`) 40.0 (`self.DynamycObjects`) null (`|MakeArray` self :!type "Actor Object Reference")))
  (bind (_outactors_2 _returnvalue_2) (`KismetSystemLibrary.SphereOverlapActors` (`self.K2_GetActorLocation`) 210.0 (`self.WorldStatycObjects`)))
  (return (or _returnvalue _returnvalue_2)))

(fn `Get Random Spawn Pos`
  (returns (SpawnPos :type "Vector Structure"))
  (return (`KismetMathLibrary.MakeVector` (`KismetMathLibrary.Conv_IntToDouble` (+ (* (`KismetMathLibrary.RandomIntegerInRange` (`self.MinCell`) (`self.MaxCell`)) 100) (.x (`self.StartCoords`)))) (`KismetMathLibrary.Conv_IntToDouble` (+ (* (`KismetMathLibrary.RandomIntegerInRange` (`self.MinCell`) (`self.MaxCell`)) 100) (.y (`self.StartCoords`)))) (`KismetMathLibrary.Conv_IntToDouble` (+ (* (`KismetMathLibrary.RandomIntegerInRange` (`self.MinCell`) (`self.MaxCell`)) 100) (.z (`self.StartCoords`)))))))

(fn `GetEnergyReward`
  (returns (EnergyReward :type "Float (double-precision)"))
  (return (`self.EnergyReward`)))

(fn `IsActorEnemy`
  (returns (IsEnemy :type Boolean))
  (return true))

(fn `IsEnemyActive`
  (returns (IsActive :type Boolean))
  (return (`self.IsActive`)))

(fn `IsEnemyInArmor`
  (returns (IsInArmor :type Boolean))
  (return (`self.IsInArmor`)))

(fn `UserConstructionScript`)