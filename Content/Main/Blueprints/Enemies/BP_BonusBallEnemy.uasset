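; Bonus ball enemy that hurts the player on contact or when its explosion countdown runs out, tracked by an on-screen compass.
; Each kill or explosion restarts the timer, shortened toward a minimum, and signals a second laser at a set threshold.
; It then hides and teleports to the farthest of several shuffled BP_BoxSpawner locations from the player, retrying via CheckSpawnSpot before revealing itself.
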(event `self.ReceiveBeginPlay`
  (`self.SetUp`)
  (`self.SetUpBonusPositions`)
  (`self.SetInitRotation` true)
  (bind _asbp_main_character (cast `/Game/Main/Blueprints/Player/BP_MainCharacter` (`GameplayStatics.GetPlayerCharacter` 0)))
  (set `self.PlayerRef` _asbp_main_character)
  (`KismetSystemLibrary.DelayUntilNextTick`)
  (`self.SpawnNewBonus`)
  (bind _returnvalue (`|CreateWidget` "/Game/Main/Blueprints/UI/WB_Compass.WB_Compass_C" (`GameplayStatics.GetPlayerController` 0)))
  (bind _output_get (set `self.Compass` _returnvalue))
  (`/Game/Main/Blueprints/UI/WB_Compass.SetCompass` _output_get (struct :`R` 0.015686 :`G` 0.65098 :`B` 0.658824 :`A` 1.0) self)
  (`UserWidget.AddToViewport` _output_get 0))

(event `self.ReceiveTick`
  (params (DeltaSeconds :type "Float (single-precision)"))
  (`self.UpdateRotation` DeltaSeconds))

(event `/Game/Main/Blueprints/Enemies/Interfaces/BPI_EnemyDeath.GetKilled`
  (`self.SpawnAfterDestroySystems`)
  (`KismetSystemLibrary.K2_ClearTimer` null "HitPlayer")
  (`self.SpawnNewBonus`))

(event `SpawnNewBonus`
  (bind _explosiontime (`self.ExplosionTime`))
  (`KismetSystemLibrary.K2_SetTimer` null "HitPlayer" (`self.ExplosionTime`))
  (`self.StartedExplosionCountdown` _explosiontime)
  (if (== _explosiontime (`self.Spawn2ndLaserTime`))
    (`self.Spawn2ndLaser`))
  (`self.DepleteExplosionTime`)
  (`self.Hide`)
  (`self.BonusRespawnIter`))

(event `HitPlayer`
  (`/Game/Main/Blueprints/Player/BP_MainCharacter.GetHurt` (`self.PlayerRef`))
  (`GameplayStatics.PlaySound2D` "/Game/Main/Audio/SFX/StarExplosion.StarExplosion" 1.0 1.0 0.0 null null)
  (`/Game/Main/Blueprints/Enemies/Interfaces/BPI_EnemyDeath.GetKilled`))

(event `BonusRespawnIter`
  (bind _bonuspos (`self.GetNewBonusPos`))
  (`self.K2_TeleportTo` _bonuspos)
  (`KismetSystemLibrary.DelayUntilNextTick`)
  (bind _isspottaken (`self.CheckSpawnSpot`))
  (if _isspottaken
    (`self.BonusRespawnIter`)
    (else
      (`self.Reveal`))))

(event `SetUpBonusPositions`
  (bind _outactors (`GameplayStatics.GetAllActorsOfClass` "/Game/Main/Blueprints/Tools/BP_BoxSpawner.BP_BoxSpawner_C"))
  (for _array_element _outactors
    (`KismetArrayLibrary.Array_Add` (`self.BonusPositions`) (`self.K2_GetActorLocation` _array_element))))

(event `self.Collider.OnComponentBeginOverlap`
  (params (OverlappedComponent :type "PrimitiveComponent Object Reference") (OtherActor :type "Actor Object Reference") (OtherComp :type "PrimitiveComponent Object Reference") (OtherBodyIndex :type Integer) (bFromSweep :type Boolean) (SweepResult :type "HitResult Structure (by ref)"))
  (bind _asbp_main_character (cast `/Game/Main/Blueprints/Player/BP_MainCharacter` OtherActor))
  (`/Game/Main/Blueprints/Player/BP_MainCharacter.GetHurt` _asbp_main_character))

(fn `DepleteExplosionTime`
  (if (> (`self.ExplosionTime`) (`self.ExplosionTimeMIn`))
    (set `self.ExplosionTime` (- (`self.ExplosionTime`) (`self.ExplosionTimeDepletion`)))))

(fn `GetFarSpotFromPlayer`
  (returns (FarPos :type "Vector Structure"))
  (locals (Counter :type Integer) (MaxDistance :type "Float (double-precision)") (Result :type "Vector Structure"))
  (while (< (`local.Counter`) (`self.MaxFarSpotCounter`))
    (`/Engine/EditorBlueprintResources/StandardMacros.IncrementInt` (`local.Counter`)
      (:`  `
        (bind _spawnpos (`self.Get Random Spawn Pos` false))
        (bind _returnvalue (`KismetMathLibrary.Vector_Distance` _spawnpos (`self.K2_GetActorLocation` (`GameplayStatics.GetPlayerCharacter` 0))))
        (if (>= _returnvalue (`local.MaxDistance`))
          (set `local.MaxDistance` _returnvalue)
          (set `local.Result` _spawnpos)))))
  (return (`local.Result`)))

(fn `GetNewBonusPos`
  (returns (BonusPos :type "Vector Structure"))
  (locals (MaxDistance :type "Float (double-precision)") (Result :type "Vector Structure") (Counter :type Integer))
  (bind _counter (`local.Counter`))
  (bind _bonuspositions (`self.BonusPositions`))
  (bind _output (`|GetArrayItem` _bonuspositions (- _counter 1)))
  (bind _returnvalue (`KismetMathLibrary.Vector_Distance` _output (`self.K2_GetActorLocation` (`GameplayStatics.GetPlayerCharacter` 0))))
  (`KismetArrayLibrary.Array_ShuffleFromStream` _bonuspositions (`KismetMathLibrary.MakeRandomStream` (`KismetMathLibrary.RandomInteger` 420)))
  (while (< (`local.Counter`) (`self.MaxBonusPosCounter`))
    (`/Engine/EditorBlueprintResources/StandardMacros.IncrementInt` _counter
      (:`  `
        (if (>= _returnvalue (`local.MaxDistance`))
          (set `local.MaxDistance` _returnvalue)
          (set `local.Result` _output)))))
  (return (`local.Result`)))

(fn `IsEnemyInArmor`
  (returns (IsInArmor :type Boolean))
  (return false))

(fn `UserConstructionScript`
  (`parent.UserConstructionScript`))