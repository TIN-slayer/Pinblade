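; Bouncing baseball enemy that flies in a random direction and exposes a score reward through GetScoreReward.
; On BeginPlay it launches its ProjectileMovement at a set speed, tilts the sphere by a random roll and picks a random spin direction.
; Each tick it spins the sphere and, whenever speed drops below the set value, rescales the normalized velocity back to it through SetVelocityInLocalSpace.
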(event `self.ReceiveBeginPlay`
  (`parent.ReceiveBeginPlay`)
  (`ProjectileMovementComponent.SetVelocityInLocalSpace` (`self.ProjectileMovement`) (* (`KismetMathLibrary.RandomUnitVector`) (`self.Velocity`)))
  (`SceneComponent.K2_SetRelativeRotation` (`self.Sphere`) (`KismetMathLibrary.MakeRotator` (`KismetMathLibrary.RandomFloatInRange` 30.0 60.0)) false false)
  (switch `int` (`KismetMathLibrary.RandomIntegerInRange` 0 1)
    (:`0`
      (set `self.RandomRotation` 1))
    (:`1`
      (set `self.RandomRotation` -1))))

(event `self.ReceiveTick`
  (params (DeltaSeconds :type "Float (single-precision)"))
  (bind _velocity (`MovementComponent.Velocity` (`self.ProjectileMovement`)))
  (`SceneComponent.K2_AddRelativeRotation` (`self.Sphere`) (`KismetMathLibrary.MakeRotator` 0.0 0.0 (* DeltaSeconds (`self.RotationVelocity`) (`self.RandomRotation`))) false false)
  (if (< (`KismetMathLibrary.VSize` _velocity) (`self.Velocity`))
    (`ProjectileMovementComponent.SetVelocityInLocalSpace` (`self.ProjectileMovement`) (* (`KismetMathLibrary.Normal` _velocity) (`self.Velocity`)))))

(fn `Get Score Reward`
  (returns (ScoreReward :type "Float (double-precision)"))
  (return (`self.ScoreReward`)))

(fn `UserConstructionScript`
  (`parent.UserConstructionScript`))