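; Laser enemy that periodically teleports to a box spawner, tracks the player with a Niagara beam and fires a charged shot.
; A looping timer respawns it at the spawner nearest the player among a shuffled sample, retrying while CheckSpawnSpot returns true.
; After activation it hurts on contact.
; Its shot warns the player, then hurts only if a line trace still hits them, while being killed cancels the laser.
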(event `ActivationPeriod`
  (`PrimitiveComponent.SetMaterial` (`self.Sphere`) 0 "/Game/Main/Materials/M_Trans.M_Trans")
  (`MeshComponent.SetOverlayMaterial` (`self.Sphere`) "/Game/Main/Materials/M_Glow.M_Glow")
  (set `self.IsActive` false)
  (`KismetSystemLibrary.Delay` (`self.ActivationTime`))
  (`PrimitiveComponent.SetMaterial` (`self.Sphere`) 0 "/Game/Main/Materials/M_Black.M_Black")
  (`MeshComponent.SetOverlayMaterial` (`self.Sphere`) "/Game/Main/Materials/M_GlowOrange.M_GlowOrange")
  (set `self.IsActive` true)
  (`FXSystemComponent.SetColorParameter` (`self.NSLaser`) "Color" (struct :`R` 1.0 :`G` 0.301961 :`A` 1.0)))

(event `self.ReceiveBeginPlay`
  (bind _additionaldelaybeforerespawntime (`self.AdditionalDelayBeforeRespawnTime`))
  (bind _delaybeforerespawntime (`self.DelayBeforeRespawnTime`))
  (`self.SetUp`)
  (`self.SetUpBoxSpawners`)
  (bind _output_get (set `self.RespawnCooldown` (+ (`self.ActivationTime`) (`self.PreChargeLaserTime`) (`self.FullChargeTime`) _delaybeforerespawntime _additionaldelaybeforerespawntime)))
  (`KismetSystemLibrary.K2_SetTimer` null "RespawnLaserEnemy" _output_get true false (- (+ _delaybeforerespawntime _additionaldelaybeforerespawntime) _output_get))
  (`self.Hide`))

(event `SetUpLaser`
  (bind _returnvalue (`NiagaraFunctionLibrary.SpawnSystemAttached` "/Game/Main/Niagara/NS_Laser.NS_Laser" (`self.Collider`) "None" (0.0 0.0 0.0) (struct) "KeepRelativeOffset"))
  (bind _output_get (set `self.NSLaser` _returnvalue))
  (`FXSystemComponent.SetColorParameter` _output_get "Color" (struct :`R` 1.0 :`G` 1.0 :`B` 1.0 :`A` 1.0)))

(event `self.Collider.OnComponentBeginOverlap`
  (params (OverlappedComponent :type "PrimitiveComponent Object Reference") (OtherActor :type "Actor Object Reference") (OtherComp :type "PrimitiveComponent Object Reference") (OtherBodyIndex :type Integer) (bFromSweep :type Boolean) (SweepResult :type "HitResult Structure (by ref)"))
  (if (`self.IsActive`)
    (bind _asbp_main_character (cast `/Game/Main/Blueprints/Player/BP_MainCharacter` OtherActor))
    (`/Game/Main/Blueprints/Player/BP_MainCharacter.GetHurt` _asbp_main_character)))

(event `TrackPlayer`
  (bind _returnvalue (- (`self.K2_GetActorLocation` (`GameplayStatics.GetPlayerCharacter` 0)) (`self.K2_GetActorLocation`)))
  (bind _outhit (`KismetSystemLibrary.LineTraceSingleByProfile` (`self.K2_GetActorLocation`) (`self.K2_GetActorLocation` (`GameplayStatics.GetPlayerCharacter` 0)) "LineTracePlayer"))
  (bind (_bblockinghit _binitialoverlap _time _distance _location _impactpoint _normal _impactnormal _physmat _hitactor) (`GameplayStatics.BreakHitResult` _outhit))
  (cast `/Game/Main/Blueprints/Player/BP_MainCharacter` _hitactor
    (:`then`
      (`NiagaraComponent.SetVariablePosition` (`self.NSLaser`) "Beam End" (- _returnvalue (* (`KismetMathLibrary.Normal` _returnvalue) 100.0) (0.0 0.0 50.0))))
    (:`CastFailed`
      (`NiagaraComponent.SetVariablePosition` (`self.NSLaser`) "Beam End" (- (- _location (`self.K2_GetActorLocation`)) (0.0 0.0 50.0))))))

(event `SetUpBoxSpawners`
  (bind _outactors (`GameplayStatics.GetAllActorsOfClass` "/Game/Main/Blueprints/Tools/BP_BoxSpawner.BP_BoxSpawner_C"))
  (for _array_element _outactors
    (bind _asbp_box_spawner (cast `/Game/Main/Blueprints/Tools/BP_BoxSpawner` _array_element))
    (`KismetArrayLibrary.Array_Add` (`self.BoxSpawners`) _asbp_box_spawner)))

(event `RespawnLaserEnemy`
  (`self.Hide`)
  (`self.LaserRespawnIter`)
  (`self.ActivationPeriod`)
  (`KismetSystemLibrary.PrintString` "LASER APPEARED" true true (struct :`R` 1.0 :`G` 0.176471 :`A` 1.0) 5.0)
  (`self.SetUpLaser`)
  (`self.FireLaser`))

(event `LaserRespawnIter`
  (bind _laserpos (`self.Get New Laser Pos`))
  (`self.K2_TeleportTo` _laserpos)
  (`KismetSystemLibrary.DelayUntilNextTick`)
  (bind _isspottaken (`self.CheckSpawnSpot`))
  (if _isspottaken
    (`self.LaserRespawnIter`)
    (else
      (`self.Reveal`))))

(event `TurnOffLaser`
  (set `self.IsLaserActive` false)
  (`KismetSystemLibrary.K2_ClearTimer` null "TrackPlayer")
  (`ActorComponent.K2_DestroyComponent` (`self.NSLaser`)))

(event `FireLaser`
  (bind _returnvalue (`GameplayStatics.GetPlayerCharacter` 0))
  (set `self.IsLaserActive` true)
  (`self.OnLaserCharge` (+ (`self.ActivationTime`) (`self.PreChargeLaserTime`) (`self.FullChargeTime`)))
  (`KismetSystemLibrary.K2_SetTimer` null "TrackPlayer" 0.0001 true true)
  (`KismetSystemLibrary.Delay` (+ (`self.ActivationTime`) (`self.PreChargeLaserTime`)))
  (if (`self.IsLaserActive`)
    (bind _asbp_main_character (cast `/Game/Main/Blueprints/Player/BP_MainCharacter` _returnvalue))
    (`/Game/Main/Blueprints/Player/BP_MainCharacter.GetLaserWarning` _asbp_main_character)
    (`KismetSystemLibrary.Delay` (`self.FullChargeTime`))
    (if (`self.IsLaserActive`)
      (bind _outhit (`KismetSystemLibrary.LineTraceSingleByProfile` (`self.K2_GetActorLocation`) (`self.K2_GetActorLocation` _returnvalue) "LineTracePlayer"))
      (bind _asbp_main_character_2 (cast `/Game/Main/Blueprints/Player/BP_MainCharacter` (`.HitActor` (`GameplayStatics.BreakHitResult` _outhit)))
        (:`then`
          (`/Game/Main/Blueprints/Player/BP_MainCharacter.GetHurt` _asbp_main_character_2))
        (:`CastFailed`
          _))
      (`GameplayStatics.PlaySound2D` "/Game/FPWeapon/Audio/FirstPersonTemplateWeaponFire02.FirstPersonTemplateWeaponFire02" 1.0 1.0 0.0 null null)
      (`self.TurnOffLaser`)
      (`KismetSystemLibrary.Delay` (`self.DelayBeforeRespawnTime`))
      (`self.Hide`))))

(event `/Game/Main/Blueprints/Enemies/BPI_EnemyDeath.GetKilled`
  (`self.SpawnAfterDestroySystems`)
  (`self.Hide`)
  (`self.TurnOffLaser`))

(fn `CanHitPlayer`
  (returns (CanHit :type Boolean))
  (if (`self.IsLaserActive`)
    (bind _outhit (`KismetSystemLibrary.LineTraceSingleByProfile` (`self.K2_GetActorLocation`) (`self.K2_GetActorLocation` (`GameplayStatics.GetPlayerCharacter` 0)) "LineTracePlayer"))
    (cast `/Game/Main/Blueprints/Player/BP_MainCharacter` (`.HitActor` (`GameplayStatics.BreakHitResult` _outhit))
      (:`then`
        (return true))
      (:`CastFailed`
        (return false)))
    (else
      (return false))))

(fn `Get New Laser Pos`
  (returns (LaserPos :type "Vector Structure"))
  (locals (Counter :type Integer) (MinDistance :type "Float (double-precision)" :default 1000000.0) (Result :type "Vector Structure"))
  (bind _counter (`local.Counter`))
  (bind _boxspawners (`self.BoxSpawners`))
  (bind _returnvalue (`self.K2_GetActorLocation` (`|GetArrayItem` _boxspawners (- _counter 1))))
  (bind _returnvalue_2 (`KismetMathLibrary.Vector_Distance` _returnvalue (`self.K2_GetActorLocation` (`GameplayStatics.GetPlayerCharacter` 0))))
  (`KismetArrayLibrary.Array_ShuffleFromStream` _boxspawners (`KismetMathLibrary.MakeRandomStream` (`KismetMathLibrary.RandomInteger` 420)))
  (while (< (`local.Counter`) (`self.MaxLaserPosCounter`))
    (`/Engine/EditorBlueprintResources/StandardMacros.IncrementInt` _counter
      (:`  `
        (if (<= _returnvalue_2 (`local.MinDistance`))
          (set `local.MinDistance` _returnvalue_2)
          (set `local.Result` _returnvalue)))))
  (return (`local.Result`)))

(fn `Get Score Reward`
  (returns (ScoreReward :type "Float (double-precision)"))
  (return (`self.ScoreReward`)))

(fn `UserConstructionScript`
  (`parent.UserConstructionScript`))