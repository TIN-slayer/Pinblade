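; BP_SpikeBallEnemy is an enemy Blueprint that hurts the main character on contact while it is active.
; Its RandomRespawn override calls the parent, makes the sphere translucent-looking with a glow overlay, disables it, then restores the black and purple-glow materials and re-arms it after a spawn timer delay.
; The collider's begin-overlap calls GetHurt on BP_MainCharacter only while the active flag is set.
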(event `self.RandomRespawn`
  (`parent.RandomRespawn`)
  (`PrimitiveComponent.SetMaterial` (`self.Sphere`) 0 "/Game/Main/Materials/M_Trans.M_Trans")
  (`MeshComponent.SetOverlayMaterial` (`self.Sphere`) "/Game/Main/Materials/M_Glow.M_Glow")
  (set `self.IsActive` false)
  (`KismetSystemLibrary.Delay` (`self.SpawnTimer`))
  (`PrimitiveComponent.SetMaterial` (`self.Sphere`) 0 "/Game/Main/Materials/M_Black.M_Black")
  (`MeshComponent.SetOverlayMaterial` (`self.Sphere`) "/Game/Main/Materials/M_GlowPurple.M_GlowPurple")
  (set `self.IsActive` true))

(event `self.Collider.OnComponentBeginOverlap`
  (params (OverlappedComponent :type "PrimitiveComponent Object Reference") (OtherActor :type "Actor Object Reference") (OtherComp :type "PrimitiveComponent Object Reference") (OtherBodyIndex :type Integer) (bFromSweep :type Boolean) (SweepResult :type "HitResult Structure (by ref)"))
  (if (`self.IsActive`)
    (bind _asbp_main_character (cast `/Game/Main/Blueprints/Player/BP_MainCharacter` OtherActor))
    (`/Game/Main/Blueprints/Player/BP_MainCharacter.GetHurt` _asbp_main_character)))

(fn `UserConstructionScript`
  (`parent.UserConstructionScript`))