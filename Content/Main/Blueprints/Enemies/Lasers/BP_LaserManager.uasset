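; BP_LaserManager controls the laser enemies in the level, periodically respawning them at random intervals.
; On BeginPlay it gathers every BP_LaserEnemy, binds to the BP_BonusBallEnemy's second-laser event and waits before the first respawn.
; RespawnLasers respawns each tracked laser and calls itself again through a random Delay placed inside the loop body.
; The bonus ball event spawns another laser at the world origin and adds it to the tracked array.
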(event `self.ReceiveBeginPlay`
  (bind _outactors (`GameplayStatics.GetAllActorsOfClass` "/Game/Main/Blueprints/Enemies/Lasers/BP_LaserEnemy.BP_LaserEnemy_C"))
  (set `self.Lasers` _outactors)
  (bind _returnvalue (`GameplayStatics.GetActorOfClass` "/Game/Main/Blueprints/Enemies/BP_BonusBallEnemy.BP_BonusBallEnemy_C"))
  (bind _output_get (set `self.BonusBallRef` _returnvalue))
  (add `/Game/Main/Blueprints/Enemies/BP_BonusBallEnemy.Spawn2ndLaser` _output_get (delegate `OnSpawn2ndLaser`))
  (`KismetSystemLibrary.Delay` (`KismetMathLibrary.RandomFloatInRange` (`self.MInRespawnLasersTime`) (`self.MaxRespawnLasersTime`)))
  (`self.RespawnLasers`))

(event `OnSpawn2ndLaser`
  (bind _returnvalue (`|SpawnActorFromClass` "/Game/Main/Blueprints/Enemies/Lasers/BP_LaserEnemy.BP_LaserEnemy_C" (`KismetMathLibrary.MakeTransform` (0.0 0.0 0.0)) "Undefined" "MultiplyWithRoot" null null))
  (`KismetArrayLibrary.Array_Add` (`self.Lasers`) _returnvalue))

(event `RespawnLasers`
  (for _array_element (`self.Lasers`)
    (`/Game/Main/Blueprints/Enemies/Lasers/BP_LaserEnemy.RespawnLaserEnemy` _array_element)
    (`KismetSystemLibrary.Delay` (`KismetMathLibrary.RandomFloatInRange` (`self.MInRespawnLasersTime`) (`self.MaxRespawnLasersTime`)))
    (`self.RespawnLasers`)))

(fn `UserConstructionScript`)