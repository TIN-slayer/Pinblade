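; Invisible spike hazard whose KillBox hurts BP_MainCharacter on overlap.
; In movable mode, set on BeginPlay or through ChangeCollision, the box uses a custom collision object channel and a hit also respawns the player through BP_MovingFloorsManager.
; When enabled, such as by KillBlueBalls, it also sends overlapping BP_BaseBallEnemy actors to a random respawn.
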(event `self.ReceiveBeginPlay`
  (if (`self.IsMovable`)
    (`self.ChangeCollision`)))

(event `self.KillBox.OnComponentBeginOverlap`
  (params (OverlappedComponent :type "PrimitiveComponent Object Reference") (OtherActor :type "Actor Object Reference") (OtherComp :type "PrimitiveComponent Object Reference") (OtherBodyIndex :type Integer) (bFromSweep :type Boolean) (SweepResult :type "HitResult Structure (by ref)"))
  (bind _asbp_main_character (cast `/Game/Main/Blueprints/Player/BP_MainCharacter` OtherActor)
    (:`then`
      (`/Game/Main/Blueprints/Player/BP_MainCharacter.GetHurt` _asbp_main_character)
      (if (`self.IsMovable`)
        (bind _returnvalue (`GameplayStatics.GetActorOfClass` "/Game/Main/Blueprints/Obstacles/MovingArena/BP_MovingFloorsManager.BP_MovingFloorsManager_C"))
        (`/Game/Main/Blueprints/Obstacles/MovingArena/BP_MovingFloorsManager.RespawnPlayer` _returnvalue)))
    (:`CastFailed`
      (if (`self.DoesKillBlueBalls`)
        (bind _asbp_base_ball_enemy (cast `/Game/Main/Blueprints/Enemies/BP_BaseBallEnemy` OtherActor))
        (`/Game/Main/Blueprints/Enemies/BP_BaseBallEnemy.RandomRespawn` _asbp_base_ball_enemy true)))))

(event `ChangeCollision`
  (`PrimitiveComponent.SetCollisionObjectType` (`self.KillBox`) "ECC_GameTraceChannel7")
  (set `self.IsMovable` true))

(event `KillBlueBalls`
  (set `self.DoesKillBlueBalls` true))

(fn `UserConstructionScript`)