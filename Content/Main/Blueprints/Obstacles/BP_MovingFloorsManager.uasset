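; Manager pawn for an endlessly rising level, moving upward at constant speed with child-actor spike floor and roof.
; At each height step it spawns walls and a pattern of polycubes, keeping two rooms alive by destroying older ones.
; On start it configures the spikes, teleports the player above a spawn block and spawns randomly placed ball enemies from the game mode's count.
; Tick's bouncing-ball loop does nothing; its movement code is disconnected.
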(event `self.ReceiveBeginPlay`
  (bind _returnvalue (`self.K2_GetActorLocation`))
  (bind _asbp_invisible_spikes (cast `/Game/Main/Blueprints/Obstacles/BP_InvisibleSpikes` (`ChildActorComponent.ChildActor` (`self.StaticSpikesFloor`))))
  (`/Game/Main/Blueprints/Obstacles/BP_InvisibleSpikes.ChangeCollision` _asbp_invisible_spikes)
  (`/Game/Main/Blueprints/Obstacles/BP_InvisibleSpikes.KillBlueBalls` _asbp_invisible_spikes)
  (bind _asbp_invisible_spikes_2 (cast `/Game/Main/Blueprints/Obstacles/BP_InvisibleSpikes` (`ChildActorComponent.ChildActor` (`self.StaticSpikesRoof`))))
  (`/Game/Main/Blueprints/Obstacles/BP_InvisibleSpikes.ChangeCollision` _asbp_invisible_spikes_2)
  (set `self.NextPoint` (.z _returnvalue))
  (`self.SpawnRoom` _returnvalue)
  (set `MovementComponent.Velocity` (`KismetMathLibrary.MakeVector` 0.0 0.0 (`self.Speed`)) (`self.FloatingPawnMovement`))
  (bind _asbp_main_character (cast `/Game/Main/Blueprints/Player/BP_MainCharacter` (`GameplayStatics.GetPlayerCharacter` 0)))
  (set `self.PlayerRef` _asbp_main_character)
  (`self.RespawnPlayer`)
  (bind _asbp_main_game_mode (cast `/Game/Main/Blueprints/Core/BP_MainGameMode` (`GameplayStatics.GetGameMode`)))
  (set `self.GameModeRef` _asbp_main_game_mode)
  (`self.SpawnSecondFloorBalls`))

(event `RespawnPlayer`
  (bind _returnvalue (`self.K2_GetActorLocation`))
  (`|SpawnActorFromClass` "/Game/Main/Blueprints/Obstacles/BP_SpawnBlock.BP_SpawnBlock_C" (`KismetMathLibrary.MakeTransform` _returnvalue) "Undefined" "MultiplyWithRoot" null null)
  (`/Game/Main/Blueprints/Player/BP_MainCharacter.TeleportMyself` (`self.PlayerRef`) (+ _returnvalue (0.0 0.0 200.0))))

(event `SpawnSecondFloorBalls`
  (for _ (range 1 (+ (`/Game/Main/Blueprints/Core/BP_MainGameMode.BlueBallCount` (`self.GameModeRef`)) 1))
    (bind _returnvalue (`|SpawnActorFromClass` "/Game/Main/Blueprints/Enemies/BP_BaseBallEnemy.BP_BaseBallEnemy_C" (`KismetMathLibrary.MakeTransform` (0.0 0.0 0.0)) "AlwaysSpawn" "MultiplyWithRoot" null null))
    (`/Game/Main/Blueprints/Enemies/BP_BaseBallEnemy.RandomRespawn` _returnvalue true)))

(event `self.ReceiveTick`
  (params (DeltaSeconds :type "Float (single-precision)"))
  (if (>= (.z (`self.K2_GetActorLocation`)) (`self.NextPoint`))
    (set `self.NextPoint` (+ (`self.NextPoint`) (`self.AdditiveHeight`)))
    (`self.SpawnRoom` (`KismetMathLibrary.MakeVector` (.x (`self.K2_GetActorLocation`)) (.y (`self.K2_GetActorLocation`)) (`self.NextPoint`))))
  (bind _outactors (`GameplayStatics.GetAllActorsOfClass` "/Game/Main/Blueprints/Enemies/BP_BouncingBaseBallEnemy.BP_BouncingBaseBallEnemy_C"))
  (for _array_element _outactors
    _))

(event `SpawnRoom`
  (params (CenterCoords :type "Vector Structure"))
  (bind _oldpolycubes (`self.OldPolycubes`))
  (bind _newpolycubes (`self.NewPolycubes`))
  (bind _oldwalls (`self.OldWalls`))
  (bind _returnvalue (`|SpawnActorFromClass` "/Game/Main/Blueprints/Obstacles/BP_Walls.BP_Walls_C" (`KismetMathLibrary.MakeTransform` CenterCoords) "Undefined" "MultiplyWithRoot" null null))
  (if (`KismetSystemLibrary.IsValid` _oldwalls)
    (`self.K2_DestroyActor` _oldwalls))
  (set `self.OldWalls` (`self.NewWalls`))
  (set `self.NewWalls` _returnvalue)
  (for (_array_element _array_index) (`self.PolycubeSpawnLocations`)
    (bind _returnvalue_2 (`|SpawnActorFromClass` "/Game/Main/Blueprints/Obstacles/BP_Polycube.BP_Polycube_C" (`KismetMathLibrary.MakeTransform` (+ CenterCoords (* _array_element (`self.PolycubeSpawnDistance`)))) "Undefined" "MultiplyWithRoot" null null))
    (if (== (`KismetArrayLibrary.Array_Length` _oldpolycubes) (`KismetArrayLibrary.Array_Length` (`self.PolycubeSpawnLocations`)))
      (`self.K2_DestroyActor` (`|GetArrayItem` _oldpolycubes _array_index)))
    (if (== (`KismetArrayLibrary.Array_Length` _newpolycubes) (`KismetArrayLibrary.Array_Length` (`self.PolycubeSpawnLocations`)))
      (`KismetArrayLibrary.Array_Set` (`self.OldPolycubes`) _array_index (`|GetArrayItem` _newpolycubes _array_index) true))
    (`KismetArrayLibrary.Array_Set` (`self.NewPolycubes`) _array_index _returnvalue_2 true)))

(fn `UserConstructionScript`)