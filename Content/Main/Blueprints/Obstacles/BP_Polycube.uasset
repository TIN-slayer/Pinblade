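; BP_Polycube is an obstacle actor that takes on a random polycube shape and orientation when play begins.
; On BeginPlay it sets the Polycube component's static mesh to a random pick from PolycubePool, then rotates the actor by a random 0–180 degree angle on each axis.
; An alternative rotation drawn from a RotationPositions array is left unconnected, and the construction script is empty.
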(event `self.ReceiveBeginPlay`
  (`StaticMeshComponent.SetStaticMesh` (`self.Polycube`) (`KismetArrayLibrary.Array_Random` (`self.PolycubePool`)))
  (`self.K2_SetActorRotation` (`KismetMathLibrary.MakeRotator` (`KismetMathLibrary.RandomFloatInRange` 0.0 180.0) (`KismetMathLibrary.RandomFloatInRange` 0.0 180.0) (`KismetMathLibrary.RandomFloatInRange` 0.0 180.0))))

(fn `UserConstructionScript`)