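; BP_Spikes is a timed spike obstacle that hurts the main character on overlap with its KillBox.
; AutoActivateSpike box-traces its location and, if something is hit, calls SpawnSpike on the game mode instead of activating.
; Activation shows the spikes as a warning, then switches materials and enables the KillBox after a delay.
; After the active time, it hides, disables collision and calls SpawnSpike again, continuing the cycle.
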(event `self.ReceiveBeginPlay`
  (bind _asbp_main_game_mode (cast `/Game/Main/Blueprints/Core/BP_MainGameMode` (`GameplayStatics.GetGameMode`)))
  (set `self.GameModeRef` _asbp_main_game_mode))

(event `AutoActivateSpike`
  (bind _returnvalue (`self.K2_GetActorLocation`))
  (`KismetSystemLibrary.DelayUntilNextTick`)
  (bind (_outhit _returnvalue_2) (`KismetSystemLibrary.BoxTraceSingleByProfile` _returnvalue _returnvalue (95.0 95.0 95.0) (struct) "SpikesProfile"))
  (if _returnvalue_2
    (`/Game/Main/Blueprints/Core/BP_MainGameMode.SpawnSpike` (`self.GameModeRef`))
    (else
      (`self.ActivateSpike`))))

(event `ActivateSpike`
  (`SceneComponent.SetVisibility` (`self.Spikes`) true false)
  (`KismetSystemLibrary.Delay` (`self.SpawnTimer`))
  (`PrimitiveComponent.SetMaterial` (`self.Spikes`) 0 "/Game/Main/Materials/M_Black.M_Black")
  (`MeshComponent.SetOverlayMaterial` (`self.Spikes`) "/Game/Main/Materials/M_GlowRed.M_GlowRed")
  (`PrimitiveComponent.SetCollisionEnabled` (`self.KillBox`) "QueryOnly")
  (set `self.IsSpikeActive` true)
  (`KismetSystemLibrary.Delay` (`self.SpikeActiveTime`))
  (`SceneComponent.SetVisibility` (`self.Spikes`) false false)
  (`PrimitiveComponent.SetMaterial` (`self.Spikes`) 0 "/Game/Main/Materials/M_Trans.M_Trans")
  (`MeshComponent.SetOverlayMaterial` (`self.Spikes`) "/Game/Main/Materials/M_GlowWhiteThick.M_GlowWhiteThick")
  (`PrimitiveComponent.SetCollisionEnabled` (`self.KillBox`) "NoCollision")
  (set `self.IsSpikeActive` false)
  (`/Game/Main/Blueprints/Core/BP_MainGameMode.SpawnSpike` (`self.GameModeRef`)))

(event `self.KillBox.OnComponentBeginOverlap`
  (params (OverlappedComponent :type "PrimitiveComponent Object Reference") (OtherActor :type "Actor Object Reference") (OtherComp :type "PrimitiveComponent Object Reference") (OtherBodyIndex :type Integer) (bFromSweep :type Boolean) (SweepResult :type "HitResult Structure (by ref)"))
  (bind _asbp_main_character (cast `/Game/Main/Blueprints/Player/BP_MainCharacter` OtherActor))
  (`/Game/Main/Blueprints/Player/BP_MainCharacter.GetHurt` _asbp_main_character))

(fn `UserConstructionScript`)