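; Manager for the moving arena: it climbs along Z, accelerating to a max speed, with spike child actors as floor and roof.
; It spawns the player on a block at start and shifts bouncing ball enemies along with its velocity.
; Each height step spawns walls and timer-staggered polycubes, deferring requests while a room is spawning.
; Old walls are destroyed, while polycubes cycle through New, Old and Bin arrays for gradual timed destruction.
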(event `self.ReceiveBeginPlay`
  (bind _returnvalue (`self.K2_GetActorLocation`))
  (bind _floatingpawnmovement (`self.FloatingPawnMovement`))
  (bind _asbp_invisible_spikes (cast `/Game/Main/Blueprints/Obstacles/BP_InvisibleSpikes` (`ChildActorComponent.ChildActor` (`self.StaticSpikesFloor`))))
  (`/Game/Main/Blueprints/Obstacles/BP_InvisibleSpikes.ChangeCollision` _asbp_invisible_spikes)
  (`/Game/Main/Blueprints/Obstacles/BP_InvisibleSpikes.KillBlueBalls` _asbp_invisible_spikes)
  (bind _asbp_invisible_spikes_2 (cast `/Game/Main/Blueprints/Obstacles/BP_InvisibleSpikes` (`ChildActorComponent.ChildActor` (`self.StaticSpikesRoof`))))
  (`/Game/Main/Blueprints/Obstacles/BP_InvisibleSpikes.ChangeCollision` _asbp_invisible_spikes_2)
  (set `self.NextPoint` (.z _returnvalue))
  (`self.SpawnRoomRequest` _returnvalue)
  (set `MovementComponent.Velocity` (`KismetMathLibrary.MakeVector` 0.0 0.0 (`self.StartingSpeed`)) (`self.FloatingPawnMovement`))
  (bind _asbp_main_character (cast `/Game/Main/Blueprints/Player/BP_MainCharacter` (`GameplayStatics.GetPlayerCharacter` 0)))
  (set `self.PlayerRef` _asbp_main_character)
  (`self.RespawnPlayer`)
  (bind _asbp_main_game_mode (cast `/Game/Main/Blueprints/Core/BP_MainGameMode` (`GameplayStatics.GetGameMode`)))
  (set `self.GameModeRef` _asbp_main_game_mode)
  (`self.SpawnSecondFloorBalls`)
  (set `FloatingPawnMovement.Acceleration` (/ (- (`self.MaxSpeed`) (`self.StartingSpeed`)) (`self.AccelerationTime`)) _floatingpawnmovement)
  (set `FloatingPawnMovement.MaxSpeed` (`self.MaxSpeed`) _floatingpawnmovement)
  (`KismetSystemLibrary.K2_SetTimer` null "ClearBinPolycubes" 0.1 true))

(event `RespawnPlayer`
  (bind _returnvalue (`self.K2_GetActorLocation`))
  (`|SpawnActorFromClass` "/Game/Main/Blueprints/Obstacles/MovingArena/BP_SpawnBlock.BP_SpawnBlock_C" (`KismetMathLibrary.MakeTransform` _returnvalue) "Undefined" "MultiplyWithRoot" null null)
  (`/Game/Main/Blueprints/Player/BP_MainCharacter.TeleportMyself` (`self.PlayerRef`) (+ _returnvalue (0.0 0.0 200.0))))

(event `SpawnSecondFloorBalls`)

(event `self.ReceiveTick`
  (params (DeltaSeconds :type "Float (single-precision)"))
  (if (>= (.z (`self.K2_GetActorLocation`)) (`self.NextPoint`))
    (set `self.NextPoint` (+ (`self.NextPoint`) (`self.AdditiveHeight`)))
    (`self.SpawnRoomRequest` (`KismetMathLibrary.MakeVector` (.x (`self.K2_GetActorLocation`)) (.y (`self.K2_GetActorLocation`)) (`self.NextPoint`))))
  (bind _outactors (`GameplayStatics.GetAllActorsOfClass` "/Game/Main/Blueprints/Enemies/BP_BouncingBaseBallEnemy.BP_BouncingBaseBallEnemy_C"))
  (for _array_element _outactors
    (`self.K2_SetActorLocation` _array_element (+ (`self.K2_GetActorLocation` _array_element) (* (`MovementComponent.Velocity` (`self.FloatingPawnMovement`)) DeltaSeconds)) false false))
  (`PawnMovementComponent.AddInputVector` (`self.FloatingPawnMovement`) (0.0 0.0 1.0) false))

(event `ClearBinPolycubes`
  (for _array_element (`self.BinPolycubes`)
    (if (`KismetSystemLibrary.IsValid` _array_element)
      (`self.K2_DestroyActor` _array_element)
      (break))))

(event `SpawnRoomRequest`
  (params (CenterCoords :type "Vector Structure"))
  (bind _output_get (set `self.RequestedCenterSpawnCoords` CenterCoords))
  (if (`self.IsRoomSpawning`)
    (`KismetSystemLibrary.K2_SetTimer` null "TryToSpawnRoom" 0.0001 true true)
    (else
      (`self.SpawnRoom` _output_get))))

(event `TryToSpawnRoom`
  (if (not (`self.IsRoomSpawning`))
    (`self.SpawnRoom` (`self.RequestedCenterSpawnCoords`))
    (`KismetSystemLibrary.K2_ClearTimer` null "TryToSpawnRoom")))

(event `SpawnRoom`
  (params (CenterCoords :type "Vector Structure"))
  (bind _oldwalls (`self.OldWalls`))
  (set `self.IsRoomSpawning` true)
  (set `self.CenterSpawnCoords` CenterCoords)
  (bind _returnvalue (`|SpawnActorFromClass` "/Game/Main/Blueprints/Obstacles/MovingArena/BP_Walls.BP_Walls_C" (`KismetMathLibrary.MakeTransform` CenterCoords) "Undefined" "MultiplyWithRoot" null null))
  (if (`KismetSystemLibrary.IsValid` _oldwalls)
    (`self.K2_DestroyActor` _oldwalls))
  (set `self.OldWalls` (`self.NewWalls`))
  (set `self.NewWalls` _returnvalue)
  (`KismetSystemLibrary.K2_SetTimer` null "SpawnPolycubes" (`self.PolycubeSpawnTime`) true true))

(event `SpawnPolycubes`
  (bind _oldpolycubes (`self.OldPolycubes`))
  (bind _newpolycubes (`self.NewPolycubes`))
  (bind _lastspawnedpolycubeindex (`self.LastSpawnedPolycubeIndex`))
  (bind _lastspawnedpolycubeindex_2 (`self.LastSpawnedPolycubeIndex`))
  (bind _returnvalue (`|SpawnActorFromClass` "/Game/Main/Blueprints/Obstacles/PolyCubes/BP_Polycube.BP_Polycube_C" (`KismetMathLibrary.MakeTransform` (+ (`self.CenterSpawnCoords`) (* (`|GetArrayItem` (`self.PolycubeSpawnLocations`) _lastspawnedpolycubeindex) (`self.PolycubeSpawnDistance`)))) "Undefined" "MultiplyWithRoot" null null))
  (if (== (`KismetArrayLibrary.Array_Length` _oldpolycubes) (`KismetArrayLibrary.Array_Length` (`self.PolycubeSpawnLocations`)))
    (`KismetArrayLibrary.Array_Set` (`self.BinPolycubes`) _lastspawnedpolycubeindex (`|GetArrayItem` _oldpolycubes _lastspawnedpolycubeindex) true))
  (if (== (`KismetArrayLibrary.Array_Length` _newpolycubes) (`KismetArrayLibrary.Array_Length` (`self.PolycubeSpawnLocations`)))
    (`KismetArrayLibrary.Array_Set` (`self.OldPolycubes`) _lastspawnedpolycubeindex (`|GetArrayItem` _newpolycubes _lastspawnedpolycubeindex) true))
  (`KismetArrayLibrary.Array_Set` (`self.NewPolycubes`) _lastspawnedpolycubeindex _returnvalue true)
  (`/Engine/EditorBlueprintResources/StandardMacros.IncrementInt` _lastspawnedpolycubeindex_2
    (:`  `
      (if (>= _lastspawnedpolycubeindex_2 (`KismetArrayLibrary.Array_Length` (`self.PolycubeSpawnLocations`)))
        (set `self.LastSpawnedPolycubeIndex` 0)
        (`KismetSystemLibrary.K2_ClearTimer` null "SpawnPolycubes")
        (set `self.IsRoomSpawning` false)))))

(fn `UserConstructionScript`)