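; Polycube obstacle whose spikes switch off in stages as the player character jumps.
; On BeginPlay it gathers its child spike actors, splits their count into three portions by percentage, and binds to the main character's jump event.
; Each jump while SpikesHP remains lowers it and deactivates the next portion of the spike array.
; ActiveSpikes re-arms a depleted cube, shuffling the array first so spikes drop in random order.
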(event `self.ReceiveBeginPlay`
  (`self.AssignSpikes`)
  (bind _asbp_main_character (cast `/Game/Main/Blueprints/Player/BP_MainCharacter` (`GameplayStatics.GetPlayerCharacter` 0)))
  (add `/Game/Main/Blueprints/Player/BP_MainCharacter.OnJump` _asbp_main_character (delegate `OnJump`)))

(event `OnJump`
  (if (> (`self.SpikesHP`) 0)
    (bind _result (`/Engine/EditorBlueprintResources/StandardMacros.DecrementInt` (`self.SpikesHP`))
      (:`  `
        (switch `int` _result
          (:`0`
            (`self.DeactivateSpikePortion` (`self.SpikesDeadOn0HP`)))
          (:`1`
            (`self.DeactivateSpikePortion` (`self.SpikesDeadOn1HP`)))
          (:`2`
            (`self.DeactivateSpikePortion` (`self.SpikesDeadOn2HP`))))))))

(event `AssignSpikes`
  (for _array_element (`self.GetAllChildActors` false)
    (bind _asbp_polycube_spikes (cast `/Game/Main/Blueprints/Obstacles/PolyCubes/BP_PolycubeSpikes` _array_element))
    (`KismetArrayLibrary.Array_Add` (`self.Spikes`) _asbp_polycube_spikes))
  (set `self.SpikesDeadOn2HP` (`KismetMathLibrary.FTrunc` (* (`KismetArrayLibrary.Array_Length` (`self.Spikes`)) (`self.SpikesDeadPercentOn2HP`))))
  (set `self.SpikesDeadOn1HP` (`KismetMathLibrary.FTrunc` (* (`KismetArrayLibrary.Array_Length` (`self.Spikes`)) (`self.SpikesDeadPercentOn1HP`))))
  (set `self.SpikesDeadOn0HP` (- (`KismetArrayLibrary.Array_Length` (`self.Spikes`)) (`self.SpikesDeadOn2HP`) (`self.SpikesDeadOn1HP`))))

(event `ActiveSpikes`
  (bind _spikes (`self.Spikes`))
  (if (== (`self.SpikesHP`) 0)
    (set `self.SpikesHP` (`self.SpikesMaxHP`))
    (set `self.LastSpikeId` 0)
    (`KismetArrayLibrary.Array_Shuffle` _spikes)
    (for _array_element _spikes
      (`/Game/Main/Blueprints/Obstacles/PolyCubes/BP_PolycubeSpikes.ActivateSpike` _array_element))))

(event `DeactivateSpikePortion`
  (params (Count :type Integer))
  (bind _lastspikeid (`self.LastSpikeId`))
  (bind _returnvalue (+ _lastspikeid Count))
  (for _index (range _lastspikeid _returnvalue)
    (`/Game/Main/Blueprints/Obstacles/PolyCubes/BP_PolycubeSpikes.DeactivateSpike` (`|GetArrayItem` (`self.Spikes`) _index)))
  (set `self.LastSpikeId` _returnvalue))

(fn `UserConstructionScript`)