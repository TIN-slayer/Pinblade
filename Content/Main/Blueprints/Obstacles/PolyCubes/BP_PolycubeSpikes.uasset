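; Polycube spike obstacle that hurts BP_MainCharacter on contact once armed.
; ActivateSpike shows four spike meshes, then after SpawnTimer, if still active, switches them to black with a red glow overlay and enables the KillBox for queries.
; DeactivateSpike hides the spikes, restores the transparent material and white glow overlay as the next warning look, and disables KillBox collision.
; KillBox overlap calls GetHurt on the character.
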(event `ActivateSpike`
  (set `self.IsActive` true)
  (`self.SetSpikesVisibility` true)
  (`KismetSystemLibrary.Delay` (`self.SpawnTimer`))
  (if (`self.IsActive`)
    (`self.SetSpikesMaterial` "/Game/Main/Materials/M_Black.M_Black")
    (`self.SetSpikesOverlayMaterial` "/Game/Main/Materials/M_GlowRed.M_GlowRed")
    (`PrimitiveComponent.SetCollisionEnabled` (`self.KillBox`) "QueryOnly")))

(event `DeactivateSpike`
  (set `self.IsActive` false)
  (`self.SetSpikesVisibility` false)
  (`self.SetSpikesMaterial` "/Game/Main/Materials/M_Trans.M_Trans")
  (`self.SetSpikesOverlayMaterial` "/Game/Main/Materials/M_GlowWhiteThick.M_GlowWhiteThick")
  (`PrimitiveComponent.SetCollisionEnabled` (`self.KillBox`) "NoCollision"))

(event `self.KillBox.OnComponentBeginOverlap`
  (params (OverlappedComponent :type "PrimitiveComponent Object Reference") (OtherActor :type "Actor Object Reference") (OtherComp :type "PrimitiveComponent Object Reference") (OtherBodyIndex :type Integer) (bFromSweep :type Boolean) (SweepResult :type "HitResult Structure (by ref)"))
  (bind _asbp_main_character (cast `/Game/Main/Blueprints/Player/BP_MainCharacter` OtherActor))
  (`/Game/Main/Blueprints/Player/BP_MainCharacter.GetHurt` _asbp_main_character))

(event `SetSpikesVisibility`
  (params (Visibility :type Boolean))
  (`SceneComponent.SetVisibility` (`self.Spikes`) Visibility false)
  (`SceneComponent.SetVisibility` (`self.Spikes1`) Visibility false)
  (`SceneComponent.SetVisibility` (`self.Spikes2`) Visibility false)
  (`SceneComponent.SetVisibility` (`self.Spikes3`) Visibility false))

(event `SetSpikesMaterial`
  (params (Material :type "MaterialInterface Object Reference"))
  (`PrimitiveComponent.SetMaterial` (`self.Spikes`) 0 Material)
  (`PrimitiveComponent.SetMaterial` (`self.Spikes1`) 0 Material)
  (`PrimitiveComponent.SetMaterial` (`self.Spikes2`) 0 Material)
  (`PrimitiveComponent.SetMaterial` (`self.Spikes3`) 0 Material))

(event `SetSpikesOverlayMaterial`
  (params (OverlayMaterial :type "MaterialInterface Object Reference"))
  (`MeshComponent.SetOverlayMaterial` (`self.Spikes`) OverlayMaterial)
  (`MeshComponent.SetOverlayMaterial` (`self.Spikes1`) OverlayMaterial)
  (`MeshComponent.SetOverlayMaterial` (`self.Spikes2`) OverlayMaterial)
  (`MeshComponent.SetOverlayMaterial` (`self.Spikes3`) OverlayMaterial))

(fn `UserConstructionScript`)